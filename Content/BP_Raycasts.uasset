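; BP_Raycasts is a debug actor that probes its surroundings with rotating line traces on the Visibility channel.
; After a Delay, Tick rotates the root, traces upward, then forward and backward behind a distance check, printing physical material and distance.
; Color-coded traces draw for one frame; the backward "<1000" message actually tests for distance below zero.
; FRaycast, uncalled here, labels impact points of two traces and holds three disconnected ones.
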(event EventBeginPlay)

(event Collision|EventActorBeginOverlap
  (params (OtherActor :type Actor%20Object%20Reference)))

(event EventTick
  (params (DeltaSeconds :type Float%20%28single-precision%29))
  (bind _defaultsceneroot (Variables|Default|GetDefaultSceneRoot))
  (bind _returnvalue (Transformation|GetWorldLocation _defaultsceneroot))
  (bind _returnvalue_2 (Transformation|GetWorldRotation _defaultsceneroot))
  (bind _returnvalue_3 (Math|Vector|GetForwardVector _returnvalue_2))
  (bind _returnvalue_4 (* _returnvalue_3 1e+04))
  (Utilities|FlowControl|Delay (Variables|Default|GetDelay))
  (Transformation|AddRelativeRotation _defaultsceneroot (Variables|Default|GetRotation) false false)
  (bind _outhit (Collision|LineTraceByChannel _returnvalue (+ _returnvalue "0,0.000000,10000.000000") "TraceTypeQuery1" false 0 "ForOneFrame" true "(R=0.983352,G=0.000000,B=1.000000,A=1.000000)"))
  (Development|PrintString (Utilities|GetDisplayName (.physmat _outhit)) true true "(R=1.000000,G=0.000000,B=0.938874,A=1.000000)")
  (Development|PrintString (Utilities|String|ToString(Float) (.distance _outhit)) true true "(R=1.000000,G=0.000000,B=0.938874,A=1.000000)")
  (if (not (> (.distance _outhit) 10001.0))
    (Utilities|FlowControl|Sequence
      (:then_0
        (bind _outhit_2 (Collision|LineTraceByChannel _returnvalue (+ _returnvalue _returnvalue_4) "TraceTypeQuery1" false 0 "ForOneFrame" true "(R=1.000000,G=0.000000,B=0.083449,A=1.000000)"))
        (Development|PrintString (Utilities|GetDisplayName (.physmat _outhit_2)) true true "(R=1.000000,G=0.000000,B=0.006910,A=1.000000)")
        (Development|PrintString (Utilities|String|ToString(Float) (.distance _outhit_2)) true true "(R=1.000000,G=0.000000,B=0.006910,A=1.000000)")
        (if (< (.distance _outhit_2) 1e+03)
          (Development|PrintString "<1000" true true "(R=1.000000,G=0.000000,B=0.153062,A=1.000000)")))
      (:then_1
        (bind _outhit_3 (Collision|LineTraceByChannel _returnvalue (- _returnvalue _returnvalue_4) "TraceTypeQuery1" false 0 "ForOneFrame" true "(R=0.000000,G=0.132313,B=1.000000,A=1.000000)"))
        (Development|PrintString (Utilities|GetDisplayName (.physmat _outhit_3)) true true "(R=0.000000,G=0.158927,B=1.000000,A=1.000000)")
        (Development|PrintString (Utilities|String|ToString(Float) (.distance _outhit_3)) true true "(R=0.000000,G=0.158927,B=1.000000,A=1.000000)")
        (if (< (.distance _outhit_3) 0.0)
          (Development|PrintString "<1000" true true "(R=0.000000,G=0.119193,B=1.000000,A=1.000000)"))))))

(fn ConstructionScript)

(fn FRaycast
  (params (NewParam :type Vector) (NewParam1 :type Vector))
  (LocalVariables|Setstart NewParam)
  (Utilities|FlowControl|Sequence
    (:then_0
      (bind _outhit (Collision|LineTraceByChannel (LocalVariables|Getstart) (Variables|Default|GetForvard) "TraceTypeQuery1" false 0 "ForOneFrame"))
      (Rendering|Debug|DrawDebugString (.impactpoint _outhit) (Utilities|String|ToString(Vector) (.impactpoint _outhit)) 0 "(R=1.000000,G=0.101256,B=0.000000,A=1.000000)"))
    (:then_4
      (bind _outhit_2 (Collision|LineTraceByChannel (LocalVariables|Getstart) (+ (Variables|/Script/Engine.SceneComponent|GetRelativeLocation (Variables|Default|GetDefaultSceneRoot)) "0.000000,0.000000,900.000000") "TraceTypeQuery1" false 0 "ForOneFrame" true "(R=0.621003,G=1.000000,B=0.000000,A=1.000000)"))
      (Rendering|Debug|DrawDebugString (.impactpoint _outhit_2) (Utilities|String|ToString(Vector) (.impactpoint _outhit_2)) 0 "(R=1.000000,G=0.906993,B=0.000000,A=1.000000)"))))